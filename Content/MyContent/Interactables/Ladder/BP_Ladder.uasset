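; BP_Ladder is an interactable actor that lets the player build a ladder in place of a placeholder cube.
; BeginPlay disables collision and tick on both stair meshes but hides only the second.
; Interacting shows that mesh, enables collision and tick on both, and hides and disables the cube.
; Overlap returns the build prompt and is interactable while BPLadderComponent is not Activated, a flag this Blueprint never sets.
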(event `/Game/MyContent/Interactables/I_InteractInterface.InteractWith`
  (params (Player :type "/Game/TopDown/Blueprints/BP_TopDownCharacter Object Reference"))
  (bind _cube (`self.Cube`))
  (bind _sm_stairs_02 (`self.SM_Stairs_02`))
  (bind _sm_stairs_01 (`self.SM_Stairs_01`))
  (`SceneComponent.SetVisibility` _sm_stairs_02 true true)
  (`PrimitiveComponent.SetCollisionEnabled` _sm_stairs_02 "QueryAndPhysics")
  (`ActorComponent.SetComponentTickEnabled` _sm_stairs_02 true)
  (`PrimitiveComponent.SetCollisionEnabled` _sm_stairs_01 "QueryAndPhysics")
  (`ActorComponent.SetComponentTickEnabled` _sm_stairs_01 true)
  (`SceneComponent.SetVisibility` _cube false true)
  (`PrimitiveComponent.SetCollisionEnabled` _cube "NoCollision")
  (`ActorComponent.SetComponentTickEnabled` _cube false))

(event `self.ReceiveBeginPlay`
  (bind _sm_stairs_02 (`self.SM_Stairs_02`))
  (bind _sm_stairs_01 (`self.SM_Stairs_01`))
  (`SceneComponent.SetVisibility` _sm_stairs_02 false true)
  (`PrimitiveComponent.SetCollisionEnabled` _sm_stairs_02 "NoCollision")
  (`ActorComponent.SetComponentTickEnabled` _sm_stairs_02 false)
  (`PrimitiveComponent.SetCollisionEnabled` _sm_stairs_01 "NoCollision")
  (`ActorComponent.SetComponentTickEnabled` _sm_stairs_01 false))

(fn `Overlap`
  (returns (interactable :type Boolean) (text :type Text))
  (return (not (`/Game/MyContent/Interactables/Ladder/BP_LadderComponent.Activated` (`self.BP_LadderComponent`))) "Press E to build a ladder"))

(fn `UserConstructionScript`)